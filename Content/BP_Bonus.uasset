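; BP_Bonus is a moving pickup that calls NewFunction0 on an overlapping BP_Pawn, then destroys itself.
; Overlapping a KillZVolume also destroys it.
; Tick prints a debug string and offsets the actor along world X, scaled by delta time.
; If that move reports a blocking hit, it spawns another BP_Bonus at the trace end without destroying itself.
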(event `self.ReceiveActorBeginOverlap`
  (params (OtherActor :type "Actor Object Reference"))
  (bind _asbp_pawn (cast `/Game/BP_Pawn` OtherActor)
    (:`then`
      (`/Game/BP_Pawn.NewFunction_0` _asbp_pawn))
    (:`CastFailed`
      (cast `KillZVolume` OtherActor)))
  (`self.K2_DestroyActor`))

(event `self.ReceiveTick`
  (params (DeltaSeconds :type "Float (single-precision)"))
  (bind _returnvalue_x (`KismetMathLibrary.BreakVector` (* (`self.Vector`) DeltaSeconds)))
  (`KismetSystemLibrary.PrintString` "Hello" true true (struct :`R` 1.0 :`G` 0.333822 :`B` 0.443788 :`A` 1.0))
  (bind _sweephitresult (`self.K2_AddActorWorldOffset` (`KismetMathLibrary.MakeVector` _returnvalue_x)))
  (bind (_bblockinghit _binitialoverlap _time _distance _location _impactpoint _normal _impactnormal _physmat _hitactor _hitcomponent _hitbonename _hititem _elementindex _faceindex _tracestart _traceend) (`GameplayStatics.BreakHitResult` _sweephitresult))
  (if _bblockinghit
    (`|SpawnActorFromClass` "BP_Bonus_C" (`KismetMathLibrary.MakeTransform` _traceend) "Undefined" "OverrideRootScale" null null)))

(fn `BP_Bonus_AutoGenFunc`
  (params (TouchedActor :type "Actor Object Reference")))

(fn `UserConstructionScript`)